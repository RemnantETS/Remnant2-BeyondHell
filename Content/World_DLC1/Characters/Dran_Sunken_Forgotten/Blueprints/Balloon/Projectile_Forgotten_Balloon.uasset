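; Balloon projectile for the Forgotten in DLC1, named for slowed falling, growing, exploding and chain explosions, though those graphs are empty here.
; Hit, hit validation and damage notifications only forward to the parent class.
; Character hit, character damage and Z-velocity checks always return false.
; Parent BeginPlay, overlap and Tick calls are disabled, leaving the Blueprint with no active logic of its own.
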(event `WorldResetInterface.OnNotifyAllWorldReset`)

(event `self.ReceiveBeginPlay`)

(event `self.ReceiveTick`
  (params (DeltaSeconds :type "Float (single-precision)")))

(event `SlowDownFall`)

(event `StopFallTimer`)

(event `StartExplode`)

(event `StartSlowDownFall`)

(event `WorldResetInterface.OnWorldReset`)

(event `StartChainExplode`)

(event `BlowUp_FX`)

(event `TweenScale`
  (params (ScaledSize :type "Float (double-precision)") (TimeToTween :type "Float (double-precision)")))

(event `self.OnProjectileHit`
  (params (Hit :type "HitResult Structure (by ref)"))
  (`parent.OnProjectileHit` Hit))

(fn `Blow Up`)

(fn `ChainExplode`
  (params (MaxChainRange :type "Float (single-precision)")))

(fn `CheckDamageForCharacters`
  (params (DamageInfo :type "DamageInfo Structure"))
  (returns (Character :type Boolean))
  (return false))

(fn `CheckHitForCharacters`
  (params (`Hit Result` :type "HitResult Structure"))
  (returns (Character :type Boolean))
  (return false))

(fn `Has-ZVelocity`
  (returns (IsFalling :type Boolean))
  (return false))

(fn `OnNotifyTakeDamage`
  (params (DamageInfo :type "DamageInfo Structure (by ref)"))
  (`parent.OnNotifyTakeDamage` DamageInfo)
  (return))

(fn `SFX_Grow`)

(fn `UserConstructionScript`)

(fn `ValidateHit`
  (params (Hit :type "HitResult Structure (by ref)") (bSimulating :type Boolean))
  (returns (ReturnValue :type Boolean))
  (bind _returnvalue (`parent.ValidateHit` Hit bSimulating))
  (return _returnvalue))