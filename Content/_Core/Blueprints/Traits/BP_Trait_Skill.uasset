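; Base trait for skills that maps its Skill item to one of the player's two ability slots.
; GetItemType picks slot 1 if the first slotted trait has this modifier, otherwise slot 2 if a second trait exists, ignoring its modifier check.
; On equip it registers that item-type override in the player inventory, then the server auto-equips the skill if owned.
; GetRelevantItemAsset exposes the Skill as the related item.
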(event `self.OnEquipped`
  (bind _out (`self.GetItemType`))
  (bind _skill (`self.Skill`))
  (bind _skill_2 (`self.Skill`))
  (bind _returnvalue (`Actor.GetComponentByClass` (`self.GetOwner`) "/Script/Remnant.RemnantPlayerInventoryComponent"))
  (`parent.OnEquipped`)
  (if (`KismetSystemLibrary.IsValidClass` _out)
    (`RemnantPlayerInventoryComponent.AddItemTypeOverride` _returnvalue _skill _out)
    (if (`KismetSystemLibrary.IsServer`)
      (if (`InventoryComponent.HasItem` _returnvalue (`|ConvertAsset` _skill) 1 -1)
        (`InventoryComponent.AutoEquipItem` _returnvalue _skill_2 false)
        (bind _asequipment (castclass `Equipment` _skill_2))
        (cast `/Game/_Core/Blueprints/Items/Skill` (`InventoryComponent.GetEquippedItemByClass` _returnvalue _asequipment))))))

(event `self.OnUnequipped`)

(event `On Added`
  (params (Result :type "InventoryResult Structure")))

(fn `GetItemType`
  (returns (Out :type "ItemType Class Reference"))
  (bind _returnvalue (`Actor.GetComponentByClass` (`self.GetOwner`) "/Script/GunfireRuntime.TraitsComponent"))
  (bind (_returnvalue_transient _returnvalue_levelmods _returnvalue_maxlevelmods _returnvalue_level _returnvalue_slotindex _returnvalue_instancedata _returnvalue_traitbp) (break `TraitInfo` (`TraitsComponent.K2_GetTraitInfoForSlot` _returnvalue 1)))
  (bind (_returnvalue_transient_2 _returnvalue_levelmods_2 _returnvalue_maxlevelmods_2 _returnvalue_level_2 _returnvalue_slotindex_2 _returnvalue_instancedata_2 _returnvalue_traitbp_2) (break `TraitInfo` (`TraitsComponent.K2_GetTraitInfoForSlot` _returnvalue 0)))
  (if (`KismetSystemLibrary.IsValidClass` _returnvalue_traitbp_2)
    (bind _astrait (cast `Trait` (`BlueprintFunctionLibraryGunfire.GetDefaultObject` _returnvalue_traitbp_2))
      (:`then`
        (bind _returnvalue_2 (`self.HasModifier` _astrait (`GameplayStatics.GetObjectClass` self)))
        (if _returnvalue_2
          (return "/Game/_Core/ItemTypes/ItemType_AbilitySlot1.ItemType_AbilitySlot1_C")
          (else
            _)))
      (:`CastFailed`
        _)))
  (if (`KismetSystemLibrary.IsValidClass` _returnvalue_traitbp)
    (bind _astrait_2 (cast `Trait` (`BlueprintFunctionLibraryGunfire.GetDefaultObject` _returnvalue_traitbp)))
    (`self.HasModifier` _astrait_2 (`GameplayStatics.GetObjectClass` self))
    (return "/Game/_Core/ItemTypes/ItemType_AbilitySlot2.ItemType_AbilitySlot2_C")))

(fn `GetRelevantItemAsset`
  (returns (ReturnValue :type "Item Class Reference"))
  (return (`self.Skill`)))

(fn `ModifyInspectInfo`
  (params (Actor :type "Actor Object Reference") (InspectLevel :type Integer) (Info :type "InspectInfo Structure (by ref)"))
  (returns (Rtn :type Boolean))
  (bind _rtn (`parent.ModifyInspectInfo` Actor InspectLevel Info))
  (return _rtn))

(fn `SlotHasMod`
  (params (Slot :type Integer))
  (returns (Out :type Boolean))
  (bind (_returnvalue_transient _returnvalue_levelmods _returnvalue_maxlevelmods _returnvalue_level _returnvalue_slotindex _returnvalue_instancedata _returnvalue_traitbp) (break `TraitInfo` (`TraitsComponent.K2_GetTraitInfoForSlot` (`Actor.GetComponentByClass` (`self.GetOwner`) "/Script/GunfireRuntime.TraitsComponent") Slot)))
  (if (`KismetSystemLibrary.IsValidClass` _returnvalue_traitbp)
    (cast `Trait` (`BlueprintFunctionLibraryGunfire.GetDefaultObject` _returnvalue_traitbp)
      (:`then`
        (return true))
      (:`CastFailed`
        _)))
  (return false))