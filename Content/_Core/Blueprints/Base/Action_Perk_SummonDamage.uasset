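; Summon-damage perk action that passes damage modification on to the perk it references.
; ModifyDamage stores the last damage info, then forwards it to DamagePerk, falling back to DamagePerkAction if no perk is valid.
; AllowAction returns true only for another summon-damage action whose valid perk, or fallback perk action, differs from its own, rejecting same-source duplicates and all other action types.
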(fn `AllowAction`
  (params (ActionBP :type "ActionBase Class Reference") (InDamageInfo :type "DamageInfo Structure (by ref)") (NewAction :type "ActionBase Object Reference"))
  (returns (ReturnValue :type Boolean))
  (bind _asaction_perk_summon_damage (cast `/Game/_Core/Blueprints/Base/Action_Perk_SummonDamage` NewAction)
    (:`then`
      (bind _damageperk (`/Game/_Core/Blueprints/Base/Action_Perk_SummonDamage.DamagePerk` _asaction_perk_summon_damage))
      (`/Engine/EditorBlueprintResources/StandardMacros.IsValid` _damageperk
        (:`Is Valid`
          (return (!= _damageperk (`self.DamagePerk`))))
        (:`Is Not Valid`
          (bind _damageperkaction (`/Game/_Core/Blueprints/Base/Action_Perk_SummonDamage.DamagePerkAction` _asaction_perk_summon_damage))
          (`/Engine/EditorBlueprintResources/StandardMacros.IsValid` _damageperkaction
            (:`Is Valid`
              (return (!= _damageperkaction (`self.DamagePerkAction`))))
            (:`Is Not Valid`
              _)))))
    (:`CastFailed`
      _))
  (return false))

(fn `ModifyDamage`
  (params (Info :type "DamageInfo Structure (by ref)"))
  (bind _damageperk (`self.DamagePerk`))
  (bind _damageperkaction (`self.DamagePerkAction`))
  (set `self.LastDamageInfo` Info)
  (`/Engine/EditorBlueprintResources/StandardMacros.IsValid` _damageperk
    (:`Is Valid`
      (`self.ModifyDamage` _damageperk Info))
    (:`Is Not Valid`
      (`/Engine/EditorBlueprintResources/StandardMacros.IsValid` _damageperkaction
        (:`Is Valid`
          (`self.ModifyDamage` _damageperkaction Info))))))