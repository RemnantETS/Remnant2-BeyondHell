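; BP_Archetype is a base archetype Blueprint that adjusts the experience its owner earns based on trait progress.
; ModifyIncomingExperience checks slot index 1 of the owner's TraitsComponent and, if that trait is valid and below MaxLevel, scales the by-ref Experience by Scalar and rounds it.
; HasTraitThatNeedsExperience performs that check, while the OnEquipped and OnLevelChanged events are empty.
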(event `self.OnEquipped`)

(event `self.OnLevelChanged`)

(fn `HasTraitThatNeedsExperience`
  (params (Traits :type "TraitsComponent Object Reference") (Index :type Integer))
  (returns (Out :type Boolean))
  (bind (_returnvalue_transient _returnvalue_levelmods _returnvalue_maxlevelmods _returnvalue_level _returnvalue_slotindex _returnvalue_instancedata _returnvalue_traitbp) (break `TraitInfo` (`TraitsComponent.GetTraitInfoForSlot` Traits Index)))
  (`/Engine/EditorBlueprintResources/StandardMacros.IsValid` Traits
    (:`Is Valid`
      (if (`KismetSystemLibrary.IsValidClass` _returnvalue_traitbp)
        (return (< _returnvalue_level (`self.MaxLevel`)))
        (else
          _)))
    (:`Is Not Valid`
      _))
  (return false))

(fn `ModifyIncomingExperience`
  (params (Experience :type "Integer (by ref)"))
  (locals (Scalar :type "Float (double-precision)" :default 0.5))
  (bind _returnvalue (`self.GetOwner`))
  (`/Engine/EditorBlueprintResources/StandardMacros.IsValid` _returnvalue
    (:`Is Valid`
      (if (`self.HasTraitThatNeedsExperience` (`Actor.GetComponentByClass` _returnvalue "/Script/GunfireRuntime.TraitsComponent") 1)
        (`|VariableSetRef` Experience (`KismetMathLibrary.Round` (* (`KismetMathLibrary.Conv_IntToDouble` Experience) (`local.Scalar`))))))))