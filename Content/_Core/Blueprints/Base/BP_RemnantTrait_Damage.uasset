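; Base Remnant trait for damage perks, which extends the trait to the owner's summons through an action and exposes an empty ModifyDamage hook.
; On equip it listens to the SummonerComponent and starts Action_Perk_SummonDamage on current and newly added summons, passing itself and its icon.
; A map tracks each summon's action, dropping entries on summon removal and stopping the actions on unequip.
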(event `self.OnUnequipped`
  (bind _summonactioninstances (`self.SummonActionInstances`))
  (`parent.OnUnequipped`)
  (remove `SummonerComponent.OnSummonAdded` (`Actor.GetComponentByClass` (`self.GetCharacter`) "/Script/Remnant.SummonerComponent") (delegate `OnSummonAdded`))
  (bind _keys (`BlueprintMapLibrary.Map_Keys` _summonactioninstances))
  (for _array_element _keys
    (`ActionComponent.StopAction` (`Actor.GetComponentByClass` _array_element "/Script/GunfireRuntime.ActionComponent") (`BlueprintMapLibrary.Map_Find` _summonactioninstances _array_element))))

(event `OnSummonRemoved`
  (params (Summon :type "Actor Object Reference"))
  (`BlueprintMapLibrary.Map_Remove` (`self.SummonActionInstances`) Summon))

(event `self.OnEquipped`
  (bind _returnvalue (`Actor.GetComponentByClass` (`self.GetCharacter`) "/Script/Remnant.SummonerComponent"))
  (`parent.OnEquipped`)
  (add `SummonerComponent.OnSummonAdded` _returnvalue (delegate `OnSummonAdded`))
  (add `SummonerComponent.OnSummonRemoved` _returnvalue (delegate `OnSummonRemoved`))
  (for _array_element (`SummonerComponent.GetSummons` _returnvalue)
    (`self.OnSummonAdded` _array_element)))

(event `OnSummonAdded`
  (params (Summon :type "Actor Object Reference"))
  (bind _returnvalue (`Actor.GetComponentByClass` Summon "/Script/GunfireRuntime.ActionComponent"))
  (bind _damageinfo (make `DamageInfo` null 0.0 0.0 0.0 1.0 1.0 0.0 0.0 0.0 -1 1.0 null (`self.GetCharacter`) Summon))
  (bind _returnvalue_2 (`|GenericCreateObject` _returnvalue "/Game/_Core/Blueprints/Base/Action_Perk_SummonDamage.Action_Perk_SummonDamage_C" self null "NewEnumerator0" -1.0 false _damageinfo 1))
  (set `ActorModifier.Icon` (`self.Icon`) _returnvalue_2)
  (bind _returnvalue_3 (`ActionComponent.CanDoActionInternal` _returnvalue "/Game/_Core/Blueprints/Base/Action_Perk_SummonDamage.Action_Perk_SummonDamage_C" _damageinfo _returnvalue_2))
  (if _returnvalue_3
    (bind _returnvalue_4 (`ActionComponent.DoActionInternal` :`self` _returnvalue :`Action` _returnvalue_2 :`DamageInfo` _damageinfo))
    (`BlueprintMapLibrary.Map_Add` (`self.SummonActionInstances`) Summon _returnvalue_4)))

(fn `ModifyDamage`
  (params (Info :type "DamageInfo Structure (by ref)")))