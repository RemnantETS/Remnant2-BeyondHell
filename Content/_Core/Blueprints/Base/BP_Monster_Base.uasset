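; BP_Monster_Base is the base monster character Blueprint, declaring the shared interface for enemy combat, spawning and loot.
; Replicated alert and combat state pairs with multicast events, alongside hooks for damage, fleeing, death stingers and contextual dialog.
; Functions cover encounters, child spawns and cleanup, modifiers, character, animation and biome tags, tag-driven loot drops, boss bar and possession setup.
; All bodies here are empty stubs, so only the interface is visible.
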(event `OnRep_OnAlerted`)

(event `OnRep_InCombat`)

(event `OnLoaded_F670E7D745B312B754269FB3F1A0F738`
  (params (Loaded :type "Object Class Reference")))

(event `OnBeginReadyWeapon`)

(event `MultiCast_OnBeginReadyWeapon`)

(event `OnAlert`)

(event `MulticastAlert`)

(event `CombatEnter`)

(event `CombatExit`)

(event `self.ReceiveBeginPlay`)

(event `DisableCollision`)

(event `EnableCollision`)

(event `OnRunAway`)

(event `UseItemInterface.UseItem`
  (params (PlayerController :type "PlayerControllerGunfire Object Reference") (ItemClass :type "Item Class Reference")))

(event `self.ReceiveEndPlay`
  (params (EndPlayReason :type "EEndPlayReason Enum" :default "Destroyed")))

(event `CleanseListedStatusEffects`)

(fn `AddAnimationTag`
  (params (Tag :type Name)))

(fn `AddCharacterTag`
  (params (Tag :type Name)))

(fn `CanUseItem`
  (params (PlayerController :type "PlayerControllerGunfire Object Reference") (ItemClass :type "Item Class Reference"))
  (returns (ReturnValue :type Boolean))
  (return false))

(fn `CleanupSpawns`
  (params (Kill :type Boolean) (Destroy :type Boolean)))

(fn `DoEncounter`
  (params (SpawnTable :type "SpawnTable Object Reference") (SpawnTag :type Name) (Rating :type Integer) (SetOwnerAsTarget :type Boolean))
  (returns (EncounterInstance :type "EncounterInstance Object Reference"))
  (return null))

(fn `DropLoot`
  (params (Cause :type "Actor Object Reference")))

(fn `DropLootAtLocation`
  (params (Location :type "Vector Structure")))

(fn `GameModeSupportsNoXPEnemies`
  (returns (Supports :type Boolean))
  (return false))

(fn `GatherContextLootDropTags`
  (params (OutTags :type "Array of Name"))
  (return))

(fn `GenerateModifier`
  (params (Tag :type Name)))

(fn `GetCauseAsCharacter`
  (params (In :type "Actor Object Reference"))
  (returns (Out :type "CharacterGunfire Object Reference"))
  (return null))

(fn `GetCombatClassNameID`
  (returns (Valid :type Boolean) (NameID :type Name))
  (return false "None"))

(fn `GetCombinedLootTags`
  (returns (OutLootTags :type "Array of Name"))
  (return))

(fn `GetEncounterMan`
  (returns (EncounterManager :type "EncounterManager Object Reference"))
  (return null))

(fn `GetScaledHealthByClass`
  (params (Prefix :type Name))
  (returns (ReturnValue :type "Float (single-precision)"))
  (return 0.0))

(fn `HasAnimTag`
  (params (AnimTag :type Name))
  (returns (ReturnValue :type Boolean))
  (return false))

(fn `HideShowMeshComponents`
  (params (HideMesh :type Boolean)))

(fn `InitializeSpawnedCharacter`
  (params (SpawnedActor :type "Actor Object Reference") (SpawnState :type Name) (AddThreat :type Boolean) (ThreatAmount :type "Float (double-precision)"))
  (returns (`AsCharacter Gunfire` :type "CharacterGunfire Object Reference"))
  (return null))

(fn `OnLoadedCharacterMods`
  (params (Classes :type "Array of Object Soft Class Reference"))
  (return))

(fn `OnNotifyTakeDamage_Event`
  (params (DamageInfo :type "DamageInfo Structure"))
  (return))

(fn `PlayAlertContextualDialog`)

(fn `PlayDeadContextualDialog`)

(fn `PlayDeathStinger`)

(fn `RemoveAnimationTag`
  (params (Tag :type Name)))

(fn `RemoveCharacterTag`
  (params (Tag :type Name)))

(fn `RunAway`)

(fn `SetAberrationBossBar`)

(fn `SetTPSHudOff`)

(fn `SetTPSHudOn`)

(fn `SetupBiomeTags`)

(fn `SetupModifiers`)

(fn `SetupPossessed`)

(fn `SoundAwareness`
  (params (Source :type "Actor Object Reference") (Radius :type "Float (double-precision)")))

(fn `SpawnCharacter`
  (params (SpawnTransform :type "Transform Structure") (ActorClass :type "Actor Class Reference") (CollisionHandling :type "ESpawnActorCollisionHandlingMethod Enum" :default "Undefined") (SpawnState :type Name) (AddThreat :type Boolean) (ThreatAmount :type "Float (double-precision)"))
  (returns (`AsCharacter Gunfire` :type "CharacterGunfire Object Reference"))
  (return null))

(fn `TryAddNoExperienceTag`)

(fn `UserConstructionScript`)