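; BP_RemnantTrait is a base Blueprint for traits, supplying inspect UI text and shared helper functions.
; ModifyInspectInfo extends the parent result, adding a custom primary "Info" stat from GetFunctionalDescription (the Description by default) when none exists.
; DoAction and DoActionOnTarget run actions through an ActionComponent, with the owning CharacterGunfire as cause.
; IsTargetAggro reports whether a pawn's AI controller has a valid current target; ModifyPreviewInfo is empty.
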(fn `DoAction`
  (params (ActionBP :type "ActionBase Class Reference"))
  (returns (ActionID :type Integer))
  (bind _out (`self.GetCharacter`))
  (if (`KismetSystemLibrary.IsValidClass` ActionBP)
    (bind _returnvalue (`ActionComponent.DoAction` :`self` (`CharacterGunfire.ActionComp` _out) :`Action` ActionBP :`Cause` _out :`Target` _out))
    (return _returnvalue)))

(fn `DoActionOnTarget`
  (params (Action :type "ActionBase Class Reference") (Target :type "Actor Object Reference"))
  (returns (ReturnValue :type Integer))
  (bind _returnvalue (`Actor.GetComponentByClass` Target "/Script/GunfireRuntime.ActionComponent"))
  (`/Engine/EditorBlueprintResources/StandardMacros.IsValid` Target
    (:`Is Valid`
      (if (`KismetSystemLibrary.IsValidClass` Action)
        (`/Engine/EditorBlueprintResources/StandardMacros.IsValid` _returnvalue
          (:`Is Valid`
            (bind _returnvalue_2 (`ActionComponent.DoAction` :`self` _returnvalue :`Action` Action :`Cause` (`self.GetCharacter`) :`Target` Target))
            (return _returnvalue_2)))))))

(fn `GetCharacter`
  (returns (Out :type "CharacterGunfire Object Reference"))
  (bind _ascharacter_gunfire (cast `CharacterGunfire` (`self.GetOwner`)))
  (return _ascharacter_gunfire))

(fn `GetFunctionalDescription`
  (params (Actor :type "Actor Object Reference") (Level :type Integer) (ReadOnlyInfo :type "InspectInfo Structure"))
  (returns (InfoText :type Text))
  (return (`self.Description`)))

(fn `IsTargetAggro`
  (params (Target :type "Actor Object Reference"))
  (returns (Out :type Boolean))
  (bind _aspawn (cast `Pawn` Target)
    (:`then`
      (bind _asaicontroller_gunfire (cast `AIControllerGunfire` (`Pawn.GetController` _aspawn))
        (:`then`
          (`/Engine/EditorBlueprintResources/StandardMacros.IsValid` (`AIControllerGunfire.GetCurrentTarget` _asaicontroller_gunfire)
            (:`Is Valid`
              (return true))
            (:`Is Not Valid`
              _)))
        (:`CastFailed`
          _)))
    (:`CastFailed`
      _))
  (return false))

(fn `ModifyInspectInfo`
  (params (Actor :type "Actor Object Reference") (InspectLevel :type Integer) (Info :type "InspectInfo Structure (by ref)"))
  (returns (Rtn :type Boolean))
  (bind _rtn (`parent.ModifyInspectInfo` Actor InspectLevel Info))
  (if (not (`.ReturnValue` (`InspectUtil.GetInspectStat` Info "Info")))
    (`InspectUtil.SetInspectStat` Info "Info" (make `InspectStat` 0.0 0.0 null "Info" "Primary" "" (`self.GetFunctionalDescription` Actor InspectLevel Info) null "Custom" 100.0)))
  (return _rtn))

(fn `ModifyPreviewInfo`
  (params (InspectInfo :type "InspectInfo Structure (by ref)")))