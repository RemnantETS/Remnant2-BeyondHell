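; Action Blueprint for a damage-over-time status effect, as named, with its graphs mostly left as stubs or pass-throughs.
; GetDamageScalar, SetDamage and AllowAction forward directly to the parent class.
; UpdateDamageScalar returns zero, while the victim lookup and longest-status-application search return nothing.
; The action start event, effect refresh and damage calculation contain no logic.
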(event `self.OnActionStart`)

(fn `AllowAction`
  (params (ActionBP :type "ActionBase Class Reference") (InDamageInfo :type "DamageInfo Structure (by ref)") (NewAction :type "ActionBase Object Reference"))
  (returns (ReturnValue :type Boolean))
  (bind _returnvalue (`parent.AllowAction` ActionBP InDamageInfo NewAction))
  (return _returnvalue))

(fn `CalculateDamage`)

(fn `FindLongestStatusApplication`
  (returns (NewParam :type "/Game/_Core/Blueprints/Actions/Action_DOT_StatusEffect Object Reference"))
  (return null))

(fn `GetDamageScalar`
  (returns (Out :type "Float (double-precision)"))
  (return (`parent.GetDamageScalar`)))

(fn `GetVictim`
  (returns (Victim :type "Actor Object Reference"))
  (return null))

(fn `RefreshEffect`
  (params (ChangeValue :type "Float (double-precision)")))

(fn `SetDamage`
  (params (TotalDamage :type "Float (double-precision)") (ApplyLevelScaling :type Boolean))
  (`parent.SetDamage` TotalDamage ApplyLevelScaling))

(fn `UpdateDamageScalar`
  (returns (EnemyType :type Byte))
  (return 0))