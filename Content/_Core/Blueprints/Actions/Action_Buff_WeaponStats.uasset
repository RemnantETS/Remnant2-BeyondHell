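; Base-style buff action that applies stat modifiers to the owner's equipped long gun and hand gun.
; On start it binds to each weapon's OnComputeStats and rebinds when either slot's item changes; on stop it unbinds both weapons.
; Each recompute feeds GetStats, empty here, into DoStatStuff, which scales stats with names ending in "Scalar" and adds the rest through ModifyStat.
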(event `OnEquippedItem`
  (params (Equipment :type "Equipment Object Reference") (ItemId :type Integer) (SlotIndex :type Integer))
  (bind _returnvalue (`Actor.GetComponentByClass` (`self.GetOwner`) "/Script/GunfireRuntime.InventoryComponent"))
  (switch `int` SlotIndex
    (:`0`
      (`self.UnbindWeaponStats` SlotIndex (`|CreateDelegate` :!event `OnComputeLongGunStats`))
      (`self.BindWeaponStats` _returnvalue SlotIndex (`|CreateDelegate` :!event `OnComputeLongGunStats`)))
    (:`1`
      (`self.UnbindWeaponStats` SlotIndex (`|CreateDelegate` :!event `OnComputeHandGunStats`))
      (`self.BindWeaponStats` _returnvalue SlotIndex (`|CreateDelegate` :!event `OnComputeHandGunStats`)))))

(event `self.OnActionStart`
  (bind _returnvalue (`Actor.GetComponentByClass` (`self.GetOwner`) "/Script/GunfireRuntime.InventoryComponent"))
  (`parent.OnActionStart`)
  (`/Engine/EditorBlueprintResources/StandardMacros.IsValid` _returnvalue
    (:`Is Valid`
      (`|ExecutionSequence`
        (:`then_0`
          (add `InventoryComponent.OnEquippedItem` _returnvalue (delegate `OnEquippedItem`)))
        (:`then_1`
          (`self.BindWeaponStats` _returnvalue 0 (`|CreateDelegate` :!event `OnComputeLongGunStats`)))
        (:`then_2`
          (`self.BindWeaponStats` _returnvalue 1 (`|CreateDelegate` :!event `OnComputeHandGunStats`)))))))

(event `self.OnActionStop`
  (`parent.OnActionStop`)
  (`|ExecutionSequence`
    (:`then_0`
      (`self.UnbindWeaponStats` 0 (`|CreateDelegate` :!event `OnComputeLongGunStats`)))
    (:`then_1`
      (`self.UnbindWeaponStats` 1 (`|CreateDelegate` :!event `OnComputeHandGunStats`)))))

(event `OnComputeLongGunStats`
  (bind _value (`BlueprintMapLibrary.Map_Find` (`self.BoundWeapons`)))
  (`self.DoStatStuff` _value (`self.GetStats` _value)))

(event `OnComputeHandGunStats`
  (bind _value (`BlueprintMapLibrary.Map_Find` (`self.BoundWeapons`) 1))
  (`self.DoStatStuff` _value (`self.GetStats` _value)))

(fn `BindWeaponStats`
  (params (InvComp :type "InventoryComponent Object Reference") (SlotIndex :type Integer) (Event :type "Delegate (by ref)"))
  (bind _returnvalue (`InventoryComponent.GetEquippedItem` InvComp SlotIndex))
  (`BlueprintMapLibrary.Map_Add` (`self.BoundWeapons`) SlotIndex _returnvalue)
  (`/Engine/EditorBlueprintResources/StandardMacros.IsValid` _returnvalue
    (:`Is Valid`
      (bind _asremnant_ranged_weapon (cast `RemnantRangedWeapon` _returnvalue))
      (bind _statscomp (`Equipment.StatsComp` _asremnant_ranged_weapon)
        (:`then`
          (add `StatsComponent.OnComputeStats` _statscomp Event)
          (`StatsComponent.Invalidate` _statscomp)
          (return))
        (:`else`)))))

(fn `DoStatStuff`
  (params (Equipment :type "Equipment Object Reference") (Stats :type "Array of InspectStat Structure"))
  (for _array_element Stats
    (bind _structout (setmembers `InspectStat` :`StructRef` _array_element))
    (if (`self.IsScalar` (`.NameID` (break `InspectStat` _structout)))
      (`Equipment.ScaleStat` Equipment (`.NameID` (break `InspectStat` _structout)) (break `InspectStat` _structout) true)
      (else
        (`Equipment.ModifyStat` Equipment (`.NameID` (break `InspectStat` _structout)) (break `InspectStat` _structout))))))

(fn `GetStats`
  (params (Equipment :type "Equipment Object Reference"))
  (returns (StatChanges :type "Array of InspectStat Structure"))
  (return))

(fn `IsScalar`
  (params (NewParam :type Name))
  (returns (ReturnValue :type Boolean))
  (return (`KismetStringLibrary.EndsWith` (`KismetStringLibrary.Conv_NameToString` NewParam) "Scalar")))

(fn `UnbindWeaponStats`
  (params (SlotIndex :type Integer) (Event :type "Delegate (by ref)"))
  (bind _value (`BlueprintMapLibrary.Map_Find` (`self.BoundWeapons`) SlotIndex))
  (`/Engine/EditorBlueprintResources/StandardMacros.IsValid` _value
    (:`Is Valid`
      (bind _asremnant_ranged_weapon (cast `RemnantRangedWeapon` _value))
      (bind _statscomp (`Equipment.StatsComp` _asremnant_ranged_weapon)
        (:`then`
          (remove `StatsComponent.OnComputeStats` _statscomp Event)
          (`StatsComponent.Invalidate` _statscomp)
          (return))
        (:`else`)))))