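; Action_Buff is a Blueprint base for buff actions, holding mostly empty stubs for reapply, lifecycle, damage, stacking and visual hooks.
; AllowAction, AllowStopAction, GetDesiredVisual and GetDebugText forward to the parent, while stack capacity always returns false and action count returns zero.
; Events, icon and visual functions have no logic, and the CharacterGunfire death binding is disconnected, so it never runs.
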(event `OnReapplyBuff`)

(event `MulticastReapplyBuff`)

(event `self.OnActionStart`)

(event `self.OnActionStop`)

(event `OnDead_Event_0`
  (params (Reason :type Byte) (Character :type "CharacterGunfire Object Reference") (Cause :type "Actor Object Reference")))

(event `self.OnTakeDamage`
  (params (DamageInfo :type "DamageInfo Structure (by ref)")))

(event `self.OnLevelChanged`)

(event `OnWorldReset`)

(fn `AllowAction`
  (params (ActionBP :type "ActionBase Class Reference") (InDamageInfo :type "DamageInfo Structure (by ref)") (NewAction :type "ActionBase Object Reference"))
  (returns (ReturnValue :type Boolean))
  (bind _returnvalue (`parent.AllowAction` ActionBP InDamageInfo NewAction))
  (return _returnvalue))

(fn `AllowStopAction`
  (returns (ReturnValue :type Boolean))
  (bind _returnvalue (`parent.AllowStopAction`))
  (return _returnvalue))

(fn `ClearVisual`)

(fn `GetActionCount`
  (returns (Out :type Integer))
  (return 0))

(fn `GetDebugText`
  (returns (ReturnValue :type String))
  (bind _returnvalue (`parent.GetDebugText`))
  (return _returnvalue))

(fn `GetDesiredVisual`
  (returns (Slot :type Name) (ID :type Name) (ReturnValue :type Boolean))
  (bind (_slot _id _returnvalue) (`parent.GetDesiredVisual`))
  (return _slot _id _returnvalue))

(fn `GetUIStackingClass`
  (returns (StackingClass :type "ActionBuff Class Reference"))
  (return null))

(fn `IsAtActionStackCapacity`
  (returns (AtMaxStacks :type Boolean))
  (return false))

(fn `SetHidden`
  (params (Hidden :type Boolean)))

(fn `SetVisual`)

(fn `UpdateIcon`)