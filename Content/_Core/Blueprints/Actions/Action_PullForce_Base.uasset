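; Base Blueprint for pull-force actions, declaring the interface for moving targets relative to an epicenter.
; It declares stubs for range and eligibility checks, epicenter location, direction and offset vectors, per-target force and force application to a character over delta time.
; All functions return zero, false or nothing and the tick event is empty, so the file itself applies no force.
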(event `self.OnTick`
  (params (DeltaSeconds :type "Float (single-precision)")))

(fn `ApplyForce`
  (params (Character :type "CharacterGunfire Object Reference") (Distance :type "Float (double-precision)") (DeltaTime :type "Float (double-precision)")))

(fn `GetEpicenterLocation`
  (returns (Location :type "Vector Structure"))
  (return (0.0 0.0 0.0)))

(fn `GetForceForActor`
  (params (Target :type "CharacterGunfire Object Reference"))
  (returns (ForceOut :type "Float (double-precision)"))
  (return 0.0))

(fn `GetOffsetVectorForActorLocation`
  (params (ActorLocation :type "Vector Structure"))
  (returns (OffsetVector :type "Vector Structure"))
  (return (0.0 0.0 0.0)))

(fn `GetToEpicenter`
  (params (TestLocation :type "Vector Structure"))
  (returns (ToEpicenter :type "Vector Structure"))
  (return (0.0 0.0 0.0)))

(fn `IsInRange`
  (params (Actor :type "Actor Object Reference"))
  (returns (ReturnValue :type Boolean))
  (return false))

(fn `ShouldMoveTarget`
  (params (Target :type "CharacterGunfire Object Reference"))
  (returns (Out :type Boolean))
  (return false))