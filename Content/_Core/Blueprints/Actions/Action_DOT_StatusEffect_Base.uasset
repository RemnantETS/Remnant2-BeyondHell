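; Base action for damage-over-time status effects, with server-set duration scaled by target and causer stats.
; It ends if the target is immune or wounded, and swaps in a fallback effect on players where disallowed.
; Player-allowed effects adjust their timer by severity, throttled on reapplication.
; Otherwise, compatible reapplications refresh the running timer instead of stacking, and a helper can duplicate the effect onto another target.
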(event `self.OnActionStart`
  (bind _returnvalue (`KismetSystemLibrary.IsServer`))
  (if _returnvalue
    (`self.ResetTimerWithNewDuration` (`self.ModifyStatusDuration` (`self.Duration`))))
  (`parent.OnActionStart`)
  (if _returnvalue
    (set `self.LastApplyTime` (`KismetSystemLibrary.GetGameTimeInSeconds`))
    (bind _ascharacter_gunfire (cast `CharacterGunfire` (`self.GetOwner`)))
    (if (`self.ShouldApplyStatus` _ascharacter_gunfire)
      (`self.VerifyValidActionForTarget`)
      (bind _returnvalue_2 (`Actor.GetComponentByClass` _ascharacter_gunfire "/Script/GunfireRuntime.WoundedComponent"))
      (`/Engine/EditorBlueprintResources/StandardMacros.IsValid` _returnvalue_2
        (:`Is Valid`
          (add `WoundedComponent.OnWounded` _returnvalue_2 (`|CreateDelegate` :!event `OnWounded`))))
      (else
        (`self.FinishAction`)))))

(fn `AllowAction`
  (params (ActionBP :type "ActionBase Class Reference") (InDamageInfo :type "DamageInfo Structure (by ref)") (NewAction :type "ActionBase Object Reference"))
  (returns (ReturnValue :type Boolean))
  (bind _returnvalue (`KismetSystemLibrary.GetGameTimeInSeconds`))
  (bind _duration (`self.Duration`))
  (if (`self.IsAllowedOnPlayer`)
    (if (> (- _returnvalue (`self.LastApplyTime`)) 0.25)
      (set `self.LastApplyTime` _returnvalue)
      (`self.ApplyTimerDelta` (- 0.0 (`self.GetPlayerSeverityValues` (`/Game/_Core/Blueprints/Actions/Action_DOT_StatusEffect_Base.PlayerSeverity` (cast `/Game/_Core/Blueprints/Actions/Action_DOT_StatusEffect_Base` NewAction :!pure true))))))
    (elif (`self.IsCompatibleAction` ActionBP InDamageInfo NewAction)
      (bind _asaction_buff (cast `/Game/_Core/Blueprints/Actions/Action_Buff` NewAction)
        (:`then`
          (bind _asaction_dot_status_effect_base (cast `/Game/_Core/Blueprints/Actions/Action_DOT_StatusEffect_Base` NewAction)
            (:`then`
              (`self.ResetTimerWithNewDuration` _duration)
              (set `self.IgnoreStatModifiers` (and (`self.IgnoreStatModifiers`) (`/Game/_Core/Blueprints/Actions/Action_DOT_StatusEffect_Base.IgnoreStatModifiers` _asaction_dot_status_effect_base))))
            (:`CastFailed`
              (`self.ResetTimerWithNewDuration` (`KismetMathLibrary.FMax` _duration (`self.ModifyStatusDuration` (`ActionBuff.Duration` _asaction_buff)))))))
        (:`CastFailed`
          (`self.ResetTimer`)))
      (else
        (return false))))
  (return false))

(fn `DuplicateStatusEffectAction`
  (params (Cause :type "Actor Object Reference") (Target :type "Actor Object Reference") (IgnoreStatModifiers :type Boolean) (IsDirectApplication :type Boolean))
  (returns (NewActionID :type Integer) (NewActionRef :type "ActionBase Object Reference"))
  (bind _returnvalue (`Actor.GetComponentByClass` Target "/Script/GunfireRuntime.ActionComponent"))
  (bind _damageinfo (make `DamageInfo` null 0.0 0.0 0.0 1.0 1.0 0.0 0.0 0.0 1.0 -1 1.0 null Cause Target))
  (bind _returnvalue_2 (`GameplayStatics.GetObjectClass` self))
  (bind _returnvalue_3 (`|GenericCreateObject` _returnvalue _returnvalue_2 "NewEnumerator0" IgnoreStatModifiers IsDirectApplication (`self.DamageType`) 0.25 (`self.Damage`) "NewEnumerator0" (`self.VisualSlot`) (`self.VisualID`) (`self.Duration`) false _damageinfo 1))
  (bind _returnvalue_4 (`ActionComponent.CanDoActionInternal` _returnvalue _returnvalue_2 _damageinfo _returnvalue_3))
  (if _returnvalue_4
    (bind _returnvalue_5 (`ActionComponent.DoActionInternal` :`self` _returnvalue :`Action` _returnvalue_3 :`DamageInfo` _damageinfo))
    (return _returnvalue_5 (`ActionComponent.GetActionByID` _returnvalue _returnvalue_5))))

(fn `GetDurationStat`
  (returns (DurationStat :type Name))
  (locals (Statuses :type "Map of /Game/_Core/Blueprints/Actions/Action_DOT_StatusEffect_Base Class Reference to Name"))
  (bind _statuses (`local.Statuses`))
  (bind _keys (`BlueprintMapLibrary.Map_Keys` _statuses))
  (for _array_element _keys
    (if (`KismetMathLibrary.ClassIsChildOf` (`GameplayStatics.GetObjectClass` self) _array_element)
      (return (`BlueprintMapLibrary.Map_Find` _statuses _array_element)))))

(fn `GetIncomingStatusEffectDurationMod`
  (returns (PlayerStatusEffectDurationMod :type "Float (single-precision)"))
  (bind _returnvalue (`self.GetActionComponent`))
  (bind _returnvalue_2 (`ActorComponent.GetOwner` _returnvalue))
  (if (not (`self.IgnoreStatModifiers`))
    (`/Engine/EditorBlueprintResources/StandardMacros.IsValid` _returnvalue
      (:`Is Valid`
        (`/Engine/EditorBlueprintResources/StandardMacros.IsValid` _returnvalue_2
          (:`Is Valid`
            (bind _ascharacter_gunfire (cast `CharacterGunfire` _returnvalue_2)
              (:`then`
                (return (`CharacterGunfire.GetStat` _ascharacter_gunfire "PlayerStatusEffectDurationMod")))
              (:`CastFailed`
                _)))
          (:`Is Not Valid`
            _)))
      (:`Is Not Valid`
        _)))
  (return 0.0))

(fn `GetOutgoingStatusEffectDurationScalar`
  (returns (EnemyStatusEffectDurationScalar :type "Float (single-precision)"))
  (bind _returnvalue (`self.GetCause`))
  (bind _durationstat (`self.GetDurationStat`))
  (bind _returnvalue_2 (`GameUtil.GetOwningCharacter` _returnvalue))
  (if (not (`self.IgnoreStatModifiers`))
    (`/Engine/EditorBlueprintResources/StandardMacros.IsValid` _returnvalue
      (:`Is Valid`
        (`/Engine/EditorBlueprintResources/StandardMacros.IsValid` _returnvalue_2
          (:`Is Valid`
            (bind _ascharacter_gunfire (cast `CharacterGunfire` _returnvalue_2)
              (:`then`
                (bind _statscomp (`CharacterGunfire.StatsComp` _ascharacter_gunfire))
                (if (`StatsComponent.HasStat` _statscomp "EnemyStatusEffectDurationScalar" false)
                  (bind _returnvalue_3 (`StatsComponent.HasStat` _statscomp _durationstat false))
                  (if _returnvalue_3
                    (bind _returnvalue_4 (`CharacterGunfire.GetStat` _ascharacter_gunfire "EnemyStatusEffectDurationScalar"))
                    (bind _returnvalue_5 (`CharacterGunfire.GetStat` _ascharacter_gunfire _durationstat))
                    (return (* _returnvalue_4 _returnvalue_5))
                    (else
                      (return _returnvalue_4)))
                  (elif _returnvalue_3
                    (return _returnvalue_5)
                    (else
                      _))))
              (:`CastFailed`
                _)))
          (:`Is Not Valid`
            _)))
      (:`Is Not Valid`
        _)))
  (return 1.0))

(fn `GetPlayerSeverityValues`
  (params (Severity :type "/Game/_Core/Blueprints/Actions/StatusEffects/EStatusEffectSeverity Enum" :default "NewEnumerator0"))
  (returns (Duration :type "Float (double-precision)"))
  (return (`MathUtil.ApplyMod` (select `byte` Severity :`0` (`self.LightSeverityTime`) :`1` (`self.MediumSeverityTime`) :`2` (`self.Duration`) :!type "Float (single-precision)") (`self.GetIncomingStatusEffectDurationMod`) 1.0)))

(fn `IsAtActionStackCapacity`
  (returns (AtMaxStacks :type Boolean))
  (return false))

(fn `IsCompatibleAction`
  (params (ActionBP :type "ActionBase Class Reference") (Damage :type "DamageInfo Structure") (NewAction :type "ActionBase Object Reference"))
  (returns (Out :type Boolean))
  (locals (Cause :type "Object Object Reference"))
  (bind _returnvalue (`self.GetCause` NewAction))
  (bind _returnvalue_2 (`self.GetCause`))
  (`|ExecutionSequence`
    (:`then_0`
      (`/Engine/EditorBlueprintResources/StandardMacros.IsValid` NewAction
        (:`Is Valid`
          (set `local.Cause` (`KismetMathLibrary.SelectObject` _returnvalue Damage_Cause (`KismetSystemLibrary.IsValid` _returnvalue))))
        (:`Is Not Valid`
          (set `local.Cause` Damage_Cause))))
    (:`then_1`
      (return (and (== (`local.Cause`) _returnvalue_2) (`KismetMathLibrary.ClassIsChildOf` (`GameplayStatics.GetObjectClass` _returnvalue_2) ActionBP))))))

(fn `ModifyStatusDuration`
  (params (Value :type "Float (single-precision)"))
  (returns (ReturnValue :type "Float (single-precision)"))
  (return (`MathUtil.ApplyMod` Value (`self.GetIncomingStatusEffectDurationMod`) (`self.GetOutgoingStatusEffectDurationScalar`))))

(fn `OnWounded`
  (params (Damage :type "DamageInfo Structure"))
  (`self.FinishAction`))

(fn `RemoveLesserEffectsOfSameType`)

(fn `ShouldApplyStatus`
  (params (self2 :type "CharacterGunfire Object Reference"))
  (returns (ReturnValue :type Boolean))
  (return (`KismetMathLibrary.BooleanNOR` (`CharacterGunfire.IsWounded` self2) (`CharacterGunfire.CheckTags` self2 (`self.ImmunityTags`) false))))

(fn `VerifyValidActionForTarget`
  (bind _returnvalue (`self.GetActionComponent`))
  (bind _returnvalue_2 (`self.GetTarget`))
  (bind _isallowedonplayer (`self.IsAllowedOnPlayer`))
  (bind _playerfallbackeffect (`self.PlayerFallbackEffect`))
  (bind _playerseverity (`self.PlayerSeverity`))
  (bind _damageinfo (make `DamageInfo` null 0.0 0.0 0.0 1.0 1.0 0.0 0.0 0.0 1.0 -1 1.0 null (`self.GetCause`) _returnvalue_2))
  (if (and (`.bSuccess` (cast `RemnantCharacter` _returnvalue_2 :!pure true)) (not _isallowedonplayer))
    (bind _returnvalue_3 (`|GenericCreateObject` _returnvalue _playerfallbackeffect _playerseverity false true (`self.DamageType`) 0.25 20.0 "NewEnumerator0" "None" "None" 5.0 false _damageinfo 1))
    (bind _returnvalue_4 (`ActionComponent.CanDoActionInternal` _returnvalue _playerfallbackeffect _damageinfo _returnvalue_3))
    (if _returnvalue_4
      (`ActionComponent.DoActionInternal` :`self` _returnvalue :`Action` _returnvalue_3 :`DamageInfo` _damageinfo)
      (`self.FinishAction`))
    (elif _isallowedonplayer
      (`self.ApplyTimerDelta` (- (`self.Duration`) (`self.GetPlayerSeverityValues` _playerseverity))))))