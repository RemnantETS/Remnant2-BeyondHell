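; Skill is an item Blueprint that outlines a character skill with charges, cooldown, duration, damage scaling, targeting and activation.
; Nearly every function and event is an empty stub or returns a default value, such as false or zero.
; Only construction, cooldown validation and cooldown reset forward to the parent class.
; Bindings to the owning character's events and state machine changes exist but are never executed.
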(event `OnActionComplete`)

(event `OnActivate`)

(event `OnSkillOwnerEvent`
  (params (EventName :type Name)))

(event `OnSkillOwnerStateChange`
  (params (StateName :type "Name (by ref)") (PreviousStateName :type "Name (by ref)")))

(event `self.OnPreApplyUseDetails`
  (params (UseType :type "EItemUseType Enum" :default "SinglePress") (OutUseDetails :type "UseDetails Structure (by ref)")))

(fn `AddCharge`)

(fn `ApplySkillChargeOverride`)

(fn `CanConsumeCharge`
  (returns (ReturnValue :type Boolean))
  (return false))

(fn `CanPlayAnimation`
  (params (Actor :type "Actor Object Reference (by ref)") (UseType :type "EItemUseType Enum (by ref)"))
  (returns (Out :type Boolean))
  (return false))

(fn `ConsumeCharge`)

(fn `DoAction`
  (params (Action :type "ActionBase Class Reference")))

(fn `GetArchetypeDamageScalar`
  (returns (Scalar :type "Float (double-precision)"))
  (return 0.0))

(fn `GetBestTargetInRange`
  (params (HostilesOnly :type Boolean) (MaxRange :type "Float (double-precision)") (ActorsToIgnore :type "Array of Actor Object Reference") (TraceRadius :type "Float (double-precision)"))
  (returns (Out :type "Actor Object Reference"))
  (return null))

(fn `GetChargesRemaining`
  (returns (Charges :type Integer))
  (return 0))

(fn `GetModifiedCooldown`
  (returns (CooldownTime :type "Float (double-precision)"))
  (return 0.0))

(fn `GetModifiedSkillDuration`
  (returns (ModifiedDuration :type "Float (double-precision)"))
  (return 0.0))

(fn `GetSkillDamageMod`
  (returns (SkillDamage :type "Float (double-precision)"))
  (return 0.0))

(fn `GetValidateUseType`
  (returns (Out :type "EItemUseType Enum"))
  (return "DoublePress"))

(fn `HasChargesForUse`
  (returns (CanUse :type Boolean))
  (return false))

(fn `HasSkillChargeOverride`
  (returns (HasOverride :type Boolean))
  (return false))

(fn `InitializeSkillCooldown`
  (params (SkipInitialCooldown :type Boolean)))

(fn `ModifySkillDuration`
  (params (Duration :type "Float (double-precision)"))
  (returns (ModifiedDuration :type "Float (double-precision)"))
  (return 0.0))

(fn `OnRep_Charges`)

(fn `OnRep_MaxCharges`)

(fn `ResetCooldown`
  (`parent.ResetCooldown`))

(fn `ShouldRefreshCooldownOnActionComplete`
  (returns (ReturnValue :type Boolean))
  (return false))

(fn `UnbindCharacterEvents`)

(fn `UpdateActiveState`)

(fn `UpdateMaxCharges`)

(fn `UserConstructionScript`
  (`parent.UserConstructionScript`))

(fn `Validate Actor Cooldown for Use`
  (params (Actor :type "Actor Object Reference"))
  (returns (Out :type Boolean))
  (bind _out (`parent.Validate Actor Cooldown for Use` Actor))
  (return _out))