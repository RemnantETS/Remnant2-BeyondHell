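; Ranged weapon mod action for multi-target aiming, with functions to find, weigh and select targets and track the projectiles assigned to them.
; Its interface covers pending and cached targets, a replication callback for pending targets, and preview indicators moved onto targets.
; Nearly all events and functions are empty stubs here, so targeting rules are not shown; CalculateClientAimVector only passes through the parent result.
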(event `OnRep_PendingTargets`)

(event `PreviewLoop`)

(event `UpdateTargets`)

(event `self.OnAttached`)

(event `self.OnDetached`)

(event `self.OnPreviewEnd`)

(event `self.ReceiveTick`
  (params (DeltaSeconds :type "Float (single-precision)")))

(event `self.OnBeginUse`)

(event `self.OnEndUse`)

(event `self.OnActivate`)

(event `self.OnPreviewStart`)

(event `CustomEvent`)

(event `self.OnDeactivate`)

(fn `AddPendingTargets`
  (params (Targets :type "Array of Actor Object Reference"))
  (return))

(fn `AddProjectile`
  (params (ForTarget :type "Actor Object Reference") (Projectile :type "Actor Object Reference")))

(fn `CalculateClientAimVector`
  (returns (AimOrigin :type "Vector Structure") (AimEnd :type "Vector Structure") (ReturnValue :type Boolean))
  (bind (_aimorigin _aimend _returnvalue) (`parent.CalculateClientAimVector`))
  (return _aimorigin _aimend _returnvalue))

(fn `ClearIndicator`
  (params (Indicator :type "Actor Object Reference")))

(fn `ClearInvalidTargets`
  (params (RemoveUnfiredProjectiles :type Boolean)))

(fn `ClearPreviewIndicators`)

(fn `ContainsValidProjectile`
  (params (Entry :type "/Game/_Core/Blueprints/Items/Mod_MultiTarget_PendingTarget Structure"))
  (returns (Out :type Boolean))
  (return false))

(fn `CreateIndicator`
  (returns (NewIndicator :type "Actor Object Reference"))
  (return null))

(fn `DrawIndicators`)

(fn `FindTargets`
  (returns (Targets :type "Array of /Game/_Core/Blueprints/Items/Mod_MultiTarget_PendingTarget Structure"))
  (return))

(fn `GetCurrentTargets`
  (params (AllowCached :type Boolean))
  (returns (Targets :type "Array of Actor Object Reference"))
  (return))

(fn `GetDrawTargets`
  (returns (Targets :type "Array of Actor Object Reference"))
  (return))

(fn `MoveIndicatorToTarget`
  (params (Indicator :type "Actor Object Reference") (Target :type "Actor Object Reference")))

(fn `OnUpdatePendingTargets`)

(fn `PickTarget`
  (params (PotentialTargets :type "Array of /Game/_Core/Blueprints/Items/Mod_MultiTarget_PendingTarget Structure"))
  (returns (Target :type Integer))
  (return 0))

(fn `RemoveProjectile`
  (params (Projectile :type "Actor Object Reference")))

(fn `SelectTargets`
  (params (PotentialTargets :type "Array of /Game/_Core/Blueprints/Items/Mod_MultiTarget_PendingTarget Structure"))
  (returns (Targets :type "Array of Actor Object Reference"))
  (return))

(fn `UpdatePreviewIndicators`)

(fn `UserConstructionScript`)

(fn `ValidateCachedTargets`)

(fn `WeighTarget`
  (params (Target :type "Actor Object Reference"))
  (returns (Weight :type "Float (double-precision)"))
  (return 0.0))