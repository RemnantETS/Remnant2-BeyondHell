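; RemnantRangedWeaponMod is a weapon mod Blueprint for ranged weapons, apparently serving as a base for specific mods.
; It declares hooks for damage, spirit and duration modifiers, plus weapon-mode preparation and clearing.
; As shown, those hooks are empty or return zero, while OnFire, CanUse and the construction script only forward to the parent class.
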(event `self.OnFire`
  (params (From :type "Vector Structure (by ref)") (To :type "Vector Structure (by ref)") (WeaponSpread :type "Float (single-precision)"))
  (`parent.OnFire` From To WeaponSpread))

(fn `CanUse`
  (params (IsSecondaryActivation :type Boolean))
  (returns (ReturnValue :type Boolean))
  (return (`parent.CanUse` IsSecondaryActivation)))

(fn `GetAllDamageMod`
  (returns (DamageMod :type "Float (double-precision)"))
  (return 0.0))

(fn `GetElementalDamageMod`
  (returns (ElementalDamageMod :type "Float (double-precision)"))
  (return 0.0))

(fn `GetExplosiveDamageMod`
  (returns (ExplosiveDamageMod :type "Float (double-precision)"))
  (return 0.0))

(fn `GetModDamageMod`
  (returns (ModDamage :type "Float (double-precision)"))
  (return 0.0))

(fn `GetModDurationMod`
  (returns (ModDurationMod :type "Float (double-precision)"))
  (return 0.0))

(fn `GetSpiritScalar`
  (returns (Out :type "Float (double-precision)"))
  (return 0.0))

(fn `GetStatusEffectDurationScalar`
  (returns (EnemyStatusEffectDurationScalar :type "Float (double-precision)"))
  (return 0.0))

(fn `GetWeaponDamageScalar`
  (returns (Out :type "Float (double-precision)"))
  (return 0.0))

(fn `ModifyModDamageInspectInfo`
  (params (Value :type "Float (single-precision)"))
  (returns (ReturnValue :type "Float (single-precision)"))
  (return 0.0))

(fn `ModifyModDuration`
  (params (Duration :type "Float (double-precision)"))
  (returns (ReturnValue :type "Float (single-precision)"))
  (return 0.0))

(fn `ModifyStatusEffectDuration`
  (params (Value :type "Float (single-precision)"))
  (returns (ReturnValue :type "Float (single-precision)"))
  (return 0.0))

(fn `PrepCharAndEquipmentForWeaponMode`)

(fn `PrepCharAndEquipmentForWeaponModeClear`)

(fn `UserConstructionScript`
  (`parent.UserConstructionScript`))