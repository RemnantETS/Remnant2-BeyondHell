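; Survival mode pickup item that awards the player the traits listed in its cached spawn list.
; PickupPreAdd loads each SpawnTableTrait entry's soft class into AllAwardedTraits, then runs the parent pickup logic.
; If the parent accepts, each trait is unlocked on the inventory owner's RemnantTraitsComponent with auto-equip allowed.
; A trait point is then added without broadcast notification and immediately used to purchase that trait.
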(fn `GetLabel`
  (returns (ReturnValue :type Text))
  (return (`parent.GetLabel`)))

(fn `PickupPreAdd`
  (params (Inventory :type "InventoryComponent Object Reference") (Quantity :type "Integer (by ref)") (Level :type Integer))
  (returns (ReturnValue :type Boolean))
  (locals (AllAwardedTraits :type "Array of Trait Class Reference"))
  (bind _cachedspawnlist_spawns (break `SpawnList` (`self.CachedSpawnList`)))
  (bind _returnvalue (`self.GetComponentByClass` (`ActorComponent.GetOwner` Inventory) "/Script/Remnant.RemnantTraitsComponent"))
  (for _array_element _cachedspawnlist_spawns
    (bind _asspawn_table_trait (cast `SpawnTableTrait` (`.Entry` (break `SpawnEntry` _array_element))))
    (bind _returnvalue_2 (`AssetUtil.LoadSoftClassReference` (`SpawnTableTrait.TraitClass` _asspawn_table_trait)))
    (bind _astrait (castclass `Trait` _returnvalue_2))
    (`KismetArrayLibrary.Array_Add` (`local.AllAwardedTraits`) _astrait))
  (bind _returnvalue_3 (`parent.PickupPreAdd` Inventory Quantity Level))
  (if _returnvalue_3
    (for _array_element_2 (`local.AllAwardedTraits`)
      (`TraitsComponent.K2_UnlockTraitSoft` :`self` _returnvalue :`TraitBP` (`|ConvertAsset` _array_element_2) :`StartingLevel` -1 :`bAllowAutoEquip` true)
      (`TraitsComponent.AddTraitPoints` _returnvalue 1 false)
      (`TraitsComponent.Purchase` _returnvalue _array_element_2))
    (return _returnvalue_3)))

(fn `UserConstructionScript`)