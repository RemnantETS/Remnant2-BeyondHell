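; BP_Curse_SpiritWisp is a spirit wisp actor for the Warlock's Curse Spirits skill, apparently a projectile.
; Each Tick calls the parent, then caches the ProjectileMovement velocity into LastVel while that component is valid.
; It adds no other logic of its own: BeginPlay and overlap events are disabled stubs, and the construction script only calls the parent.
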(event `self.ReceiveTick`
  (params (DeltaSeconds :type "Float (single-precision)"))
  (bind _projectilemovement (`self.ProjectileMovement`))
  (`parent.ReceiveTick` DeltaSeconds)
  (`/Engine/EditorBlueprintResources/StandardMacros.IsValid` _projectilemovement
    (:`Is Valid`
      (set `self.LastVel` (`MovementComponent.Velocity` _projectilemovement)))))

(fn `UserConstructionScript`
  (`parent.UserConstructionScript`))