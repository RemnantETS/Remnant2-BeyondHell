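; Post-process ground aura VFX actor for the Chronomancer's Time Jump skill.
; On BeginPlay it adds a dynamic aura material to its post-process component, plays an attached blast sound and sets origin and size from its location and Radius a tick later.
; Tweens animate a Fade float, which looping timers copy to the material to expand the radius, then fade alpha after a delay, each clearing at its limit.
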(event `self.ReceiveBeginPlay`
  (bind _dmi_groundaura (`self.DMI_GroundAura`))
  (`|ExecutionSequence`
    (:`then_0`
      (bind _returnvalue (`KismetMaterialLibrary.CreateDynamicMaterialInstance` "/Game/World_ETS/Items/Archetypes/Chronomancer/Skills/TimeJump/VFX/Material/PPM_TimeJump_Aura.PPM_TimeJump_Aura"))
      (bind _output_get (set `self.DMI_GroundAura` _returnvalue))
      (set `PostProcessComponent.Settings` (make `PostProcessSettings` :`WeightedBlendables` (make `WeightedBlendables` (`|MakeArray` (make `WeightedBlendable` 1.0 _output_get)))) (`self.PP_GroundAura`)))
    (:`then_1`
      (`TweenComponent.AnimateFloatProperty` (`self.Tween`) self "Fade" 0.0 1.05 1.0 "EaseIn" 2.0)
      (bind _returnvalue_2 (`KismetSystemLibrary.K2_SetTimerDelegate` (`|CreateDelegate` :!event `FadeInEvent`) 0.05 true))
      (set `self.FadeInTimer` _returnvalue_2)
      (`KismetSystemLibrary.Delay` 1.5)
      (`TweenComponent.AnimateFloatProperty` (`self.Tween`) self "Fade" 1.0 0.0 2.0 "EaseOut" 2.0)
      (bind _returnvalue_3 (`KismetSystemLibrary.K2_SetTimerDelegate` (`|CreateDelegate` :!event `FadeOutEvent`) 0.05 true))
      (set `self.FadeOutTimer` _returnvalue_3))
    (:`then_2`
      (`KismetSystemLibrary.DelayUntilNextTick`)
      (`MaterialInstanceDynamic.SetVectorParameterValue` _dmi_groundaura "Origin" (`KismetMathLibrary.Conv_VectorToLinearColor` (`self.K2_GetActorLocation`)))
      (`MaterialInstanceDynamic.SetScalarParameterValue` _dmi_groundaura "Size" (* (`self.Radius`) 3.2)))
    (:`then_3`
      (`GunfireAudioSystem.SpawnSoundAttached` (make `SoundGunfire` "/Game/WwiseAudio/Events/Player/Player_Archetypes_DLC1/DLC1_Ritualist/DLC1_Archetype_Ritualist_Miasma_Blast.DLC1_Archetype_Ritualist_Miasma_Blast") (`self.PP_GroundAura`)))))

(event `FadeInEvent`
  (`MaterialInstanceDynamic.SetScalarParameterValue` (`self.DMI_GroundAura`) "Radius" (* (`self.Radius`) (`self.Fade`) 1.2))
  (if (> (`self.Fade`) 1.0)
    (`KismetSystemLibrary.K2_ClearAndInvalidateTimerHandle` (`self.FadeInTimer`))))

(event `FadeOutEvent`
  (`MaterialInstanceDynamic.SetScalarParameterValue` (`self.DMI_GroundAura`) "Alpha" (`self.Fade`))
  (if (<= (`self.Fade`) 0.0)
    (`KismetSystemLibrary.K2_ClearAndInvalidateTimerHandle` (`self.FadeOutTimer`))))

(fn `UserConstructionScript`)