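; Stacking Frigid debuff action that slows its owner and raises the crit chance of incoming damage per stack level.
; It starts a linked slow action, stops it on end, and resets its timer on reapply.
; A Hailstone tag on the causing equipment's wielder doubles max stacks and converts a full stack to Frostbyte.
; AllowAction gives player targets plain Frigid instead and otherwise blocks stacking during the StasisBeam debuff.
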(event `self.OnReapplyBuff`
  (`self.ResetTimer`))

(event `self.OnActionStart`
  (bind _damageinfo (make `DamageInfo` null 0.0 0.0 0.0 1.0 1.0 0.0 0.0 0.0 -1 1.0 null (`self.GetCause`) (`self.GetOwner`)))
  (`parent.OnActionStart`)
  (`|ExecutionSequence`
    (:`then_0`
      (if (`self.HasHailstone`)
        (set `self.MaxStackCount` (* (`self.MaxStackCount`) 2))))
    (:`then_1`
      (bind _ascharacter_gunfire (cast `CharacterGunfire` (`self.GetOwner`)))
      (bind _actioncomp (`CharacterGunfire.ActionComp` _ascharacter_gunfire))
      (bind _returnvalue (`|GenericCreateObject` _actioncomp "/Game/_Core/Blueprints/Actions/Status_Slow/Action_Slow_Player.Action_Slow_Player_C" 1 "Frigid" "NewEnumerator0" -1.0 false _damageinfo))
      (bind _returnvalue_2 (`ActionComponent.CanDoActionInternal` _actioncomp "/Game/_Core/Blueprints/Actions/Status_Slow/Action_Slow_Player.Action_Slow_Player_C" _damageinfo _returnvalue))
      (if _returnvalue_2
        (bind _returnvalue_3 (`ActionComponent.DoActionInternal` :`self` _actioncomp :`Action` _returnvalue :`DamageInfo` _damageinfo))
        (set `self.SlowID` _returnvalue_3)))))

(event `self.OnActionStop`
  (`parent.OnActionStop`)
  (bind _ascharacter_gunfire (cast `CharacterGunfire` (`self.GetOwner`)))
  (`ActionComponent.StopAction` (`CharacterGunfire.ActionComp` _ascharacter_gunfire) (`self.SlowID`)))

(fn `AllowAction`
  (params (ActionBP :type "ActionBase Class Reference") (InDamageInfo :type "DamageInfo Structure (by ref)") (NewAction :type "ActionBase Object Reference"))
  (returns (ReturnValue :type Boolean))
  (bind _returnvalue (`parent.AllowAction` ActionBP InDamageInfo NewAction))
  (if (`self.IsPlayer`)
    (`self.DoAction` "/Game/World_Base/Affixes/Stat/Frigid/Action_Frigid.Action_Frigid_C")
    (`self.FinishAction`)
    (elif (`self.HasHailstone`)
      (if (== (`self.Level`) (`self.MaxStackCount`))
        (`self.DoAction` "/Game/World_ETS/Blueprints/Actions/Action_Debuff_Frostbyte.Action_Debuff_Frostbyte_C")
        (`self.FinishAction`)
        (else
          (return (and (not (`ActionComponent.IsActionTypeRunning` (`self.GetActionComponent`) "/Game/World_Nerud/Items/Mods/StasisBeam/Action_Mod_StasisBeam_Debuff.Action_Mod_StasisBeam_Debuff_C")) _returnvalue))))
      (else
        (return (and (not (`ActionComponent.IsActionTypeRunning` (`self.GetActionComponent`) "/Game/World_Nerud/Items/Mods/StasisBeam/Action_Mod_StasisBeam_Debuff.Action_Mod_StasisBeam_Debuff_C")) _returnvalue))))))

(fn `DoAction`
  (params (ActionBP :type "ActionBuff Class Reference"))
  (bind _damageinfo (make `DamageInfo` null 0.0 0.0 0.0 1.0 1.0 0.0 0.0 0.0 -1 1.0 null (`self.GetCause`) (`self.GetOwner`)))
  (bind _ascharacter_gunfire (cast `CharacterGunfire` (`self.GetOwner`)))
  (bind _actioncomp (`CharacterGunfire.ActionComp` _ascharacter_gunfire))
  (bind _returnvalue (`ActionComponent.CanDoActionInternal` _actioncomp ActionBP _damageinfo null))
  (if _returnvalue
    (bind _returnvalue_2 (`|GenericCreateObject` _actioncomp ActionBP (`self.StasisDuration`) false _damageinfo))
    (`ActionComponent.DoActionInternal` :`self` _actioncomp :`Action` _returnvalue_2 :`DamageInfo` _damageinfo)))

(fn `HasHailstone`
  (returns (ReturnValue :type Boolean))
  (bind _asequipment (cast `Equipment` (`self.GetCause`))
    (:`then`
      (bind _asremnant_character (cast `RemnantCharacter` (`Equipment.GetCharacter` _asequipment))
        (:`then`
          (return (`CharacterGunfire.CheckTag` _asremnant_character "Hailstone")))
        (:`CastFailed`
          _)))
    (:`CastFailed`
      _))
  (return false))

(fn `IsPlayer`
  (returns (Out :type Boolean))
  (return (`.bSuccess` (cast `RemnantCharacter` (`self.GetOwner`) :!pure true))))

(fn `ModifyIncomingDamage`
  (params (Info :type "DamageInfo Structure (by ref)"))
  (`DamageInfoUtil.ModifyCrit` Info (* (`self.Level`) (`self.CritChance`))))