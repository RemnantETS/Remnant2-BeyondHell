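; Frostbyte debuff action that deals damage over time to its owner and builds Frigid stacks on it.
; A looping one-second timer applies Frostbyte DOT damage, then attempts a stacking Frigid debuff through the owner's ActionComp.
; It attempts a second stack per tick when the causing equipment's wielder has the Hailstone tag.
; Reapplying calls ResetTimer, and stopping clears the tick timer.
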(event `self.OnActionStart`
  (`parent.OnActionStart`)
  (bind _returnvalue (`KismetSystemLibrary.K2_SetTimerDelegate` (delegate `ApplyFrigid`) 1.0 true))
  (set `self.TimerHandle` _returnvalue))

(event `ApplyFrigid`
  (`self.DoDamage`)
  (`self.DoFrigidStack`)
  (if (`self.HasHailstone`)
    (`self.DoFrigidStack`)))

(event `self.OnReapplyBuff`
  (`self.ResetTimer`))

(event `self.OnActionStop`
  (`parent.OnActionStop`)
  (`KismetSystemLibrary.K2_ClearAndInvalidateTimerHandle` (`self.TimerHandle`)))

(fn `DoDamage`
  (`CombatUtil.ApplyDamage` (`self.GetCause`) (`self.GetOwner`) (`self.Damage`) 0.0 1.0 11 "/Game/_Core/DamageTypes/DamageType_DOT_Frostbyte.DamageType_DOT_Frostbyte_C"))

(fn `DoFrigidStack`
  (bind _damageinfo (make `DamageInfo` null 0.0 0.0 0.0 1.0 1.0 0.0 0.0 0.0 -1 1.0 null (`self.GetCause`) (`self.GetOwner`)))
  (bind _ascharacter_gunfire (cast `CharacterGunfire` (`self.GetOwner`)))
  (bind _actioncomp (`CharacterGunfire.ActionComp` _ascharacter_gunfire))
  (bind _returnvalue (`ActionComponent.CanDoActionInternal` _actioncomp "/Game/World_ETS/Blueprints/Actions/Action_Debuff_Frigid_Stacking.Action_Debuff_Frigid_Stacking_C" _damageinfo null))
  (if _returnvalue
    (bind _returnvalue_2 (`|GenericCreateObject` _actioncomp "/Game/World_ETS/Blueprints/Actions/Action_Debuff_Frigid_Stacking.Action_Debuff_Frigid_Stacking_C" "NewEnumerator1" 20.0 false _damageinfo))
    (`ActionComponent.DoActionInternal` :`self` _actioncomp :`Action` _returnvalue_2 :`DamageInfo` _damageinfo)))

(fn `HasHailstone`
  (returns (ReturnValue :type Boolean))
  (bind _asequipment (cast `Equipment` (`self.GetCause`))
    (:`then`
      (bind _asremnant_character (cast `RemnantCharacter` (`Equipment.GetCharacter` _asequipment))
        (:`then`
          (return (`CharacterGunfire.CheckTag` _asremnant_character "Hailstone")))
        (:`CastFailed`
          _)))
    (:`CastFailed`
      _))
  (return false))