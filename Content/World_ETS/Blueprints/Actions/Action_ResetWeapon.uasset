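; Weapon action that resets a weapon by removing it from its inventory and adding it back.
; On start it binds to the weapon's unequipped event, then removes the item by class, quantity and level.
; When that event fires, it waits briefly, soft-adds the same item with forced equip and a notification, then finishes the action.
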(event `self.OnActionStart`
  (bind _weapon (`self.Weapon`))
  (add `Equipment.OnUnequippedEvent` _weapon (delegate `OnRemoved`))
  (bind _output_get (set `self.Inventory` (`Equipment.GetInventoryComponent` _weapon)))
  (`InventoryComponent.RemoveItem` _output_get (`self.Item`) (`self.Count`) (`self.ItemLevel`)))

(event `OnRemoved`
  (params (Equipment :type "Equipment Object Reference"))
  (`KismetSystemLibrary.Delay` 0.2)
  (`InventoryComponent.K2_AddItemSoft` :`self` (`self.Inventory`) :`ItemBP` (`self.Item`) :`Quantity` (`self.Count`) :`ItemLevel` (`self.ItemLevel`) :`Reason` "Default" :`ForceEquip` true :`SendNotification` true)
  (`self.FinishAction`))