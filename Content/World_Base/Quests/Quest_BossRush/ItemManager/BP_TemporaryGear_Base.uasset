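; Base pickup for temporary gear in the Boss Rush quest, awarding one item to the collector and random gear to other players.
; It trims each cached spawn list to its first entry on BeginPlay and again on award.
; An item manager action, started on the character's ActionComponent, receives the awarded spawn list when removal registration is enabled.
; On pickup, other players' item managers each receive a separately generated item from RandomizedDrop.
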(event `self.ReceiveBeginPlay`
  (`self.FilterSpawnInfo`)
  (`parent.ReceiveBeginPlay`))

(event `self.OnPickedUp`
  (params (Inventory :type "InventoryComponent Object Reference"))
  (`self.SharePickup` Inventory)
  (`parent.OnPickedUp` Inventory))

(fn `FilterSpawnInfo`
  (bind _cachedspawninfo (`self.CachedSpawnInfo`))
  (`|ExecutionSequence`
    (:`then_0`
      (if (`KismetArrayLibrary.Array_IsEmpty` (`self.TempSpawnInfo`))
        (set `self.TempSpawnInfo` _cachedspawninfo)))
    (:`then_1`
      (for (_ _array_index) _cachedspawninfo
        (bind (_output_hastarget _output_target _output_targetishost _output_cachedspawnlist) (break `GenericDropInfo` (`|GetArrayItem` _cachedspawninfo _array_index)))
        (`self.FilterSpawnList` _output_cachedspawnlist)))))

(fn `FilterSpawnList`
  (params (SpawnList :type "SpawnList Structure (by ref)"))
  (bind _spawns (break `SpawnList` SpawnList))
  (if (`KismetArrayLibrary.Array_IsNotEmpty` _spawns)
    (setmembers `SpawnList` :`StructRef` SpawnList :`Spawns` (`|MakeArray` (`|GetArrayItem` _spawns)))))

(fn `GenerateRandomItem`
  (returns (Item :type "Item Class Reference"))
  (bind _spawnlist (`SpawnTable.Generate` (`self.RandomizedDrop`) 0 0 (`self.SpawnTags`) "All"))
  (bind (_output_type _output_actorbp _output_actortags _output_spawnfaction _output_cachedactorbp _output_level _output_quantity _output_spawnpointtags _output_spawnflags _output_entry) (break `SpawnEntry` (`|GetArrayItem` (break `SpawnList` _spawnlist))))
  (bind _asspawn_table_item (cast `SpawnTableItem` _output_entry))
  (bind _returnvalue (`AssetUtil.LoadSoftClassReference` (`SpawnTableItem.ItemBP` _asspawn_table_item)))
  (bind _asitem (castclass `Item` _returnvalue))
  (return _asitem))

(fn `GetControllerFromInventoryComponent`
  (params (Inventory :type "InventoryComponent Object Reference"))
  (returns (Controller :type "PlayerController Object Reference"))
  (bind _asremnant_character (cast `RemnantCharacter` (`ActorComponent.GetOwner` Inventory)))
  (bind _asplayer_controller (cast `PlayerController` (`Pawn.GetController` _asremnant_character)))
  (return _asplayer_controller))

(fn `GetItemManager`
  (params (Actor :type "Actor Object Reference"))
  (returns (ItemManager :type "/Game/World_Base/Quests/Quest_BossRush/ItemManager/Action_Temporary_ItemManager Object Reference"))
  (bind _returnvalue (`self.GetComponentByClass` Actor "/Script/GunfireRuntime.ActionComponent"))
  (`/Engine/EditorBlueprintResources/StandardMacros.IsValid` Actor
    (:`Is Valid`
      (`/Engine/EditorBlueprintResources/StandardMacros.IsValid` _returnvalue
        (:`Is Valid`
          (`ActionComponent.DoAction` :`self` _returnvalue :`Action` "/Game/World_Base/Quests/Quest_BossRush/ItemManager/Action_Temporary_ItemManager.Action_Temporary_ItemManager_C" :`Cause` Actor :`Target` Actor)
          (bind _asaction_temporary_item_manager (cast `/Game/World_Base/Quests/Quest_BossRush/ItemManager/Action_Temporary_ItemManager` (`ActionComponent.GetActionOfType` _returnvalue "/Game/World_Base/Quests/Quest_BossRush/ItemManager/Action_Temporary_ItemManager.Action_Temporary_ItemManager_C"))
            (:`then`
              (return _asaction_temporary_item_manager))
            (:`CastFailed`
              _)))
        (:`Is Not Valid`
          _)))
    (:`Is Not Valid`
      _))
  (return null))

(fn `HandleAward`
  (params (Inventory :type "InventoryComponent Object Reference") (bForceNoSharing :type Boolean))
  (locals (TempList :type "Array of Item Soft Class Reference"))
  (bind _cachedspawnlist (`self.CachedSpawnList`))
  (`|ExecutionSequence`
    (:`then_0`
      (`self.FilterSpawnList` _cachedspawnlist)
      (if (`self.RegisterItemForRemoval`)
        (bind _itemmanager (`self.GetItemManager` (`ActorComponent.GetOwner` Inventory)))
        (`/Game/World_Base/Quests/Quest_BossRush/ItemManager/Action_Temporary_ItemManager.BreakSpawnList` _itemmanager _cachedspawnlist)))
    (:`then_1`
      (`parent.HandleAward` Inventory bForceNoSharing))))

(fn `SharePickup`
  (params (PickupInventory :type "InventoryComponent Object Reference"))
  (bind _returnvalue (`GameUtil.GetPlayerControllers`))
  (for _array_element _returnvalue
    (if (!= _array_element (`self.GetControllerFromInventoryComponent` PickupInventory))
      (bind _asremnant_player_controller (cast `RemnantPlayerController` _array_element))
      (bind _itemmanager (`self.GetItemManager` (`Controller.K2_GetPawn` _asremnant_player_controller)))
      (`/Game/World_Base/Quests/Quest_BossRush/ItemManager/Action_Temporary_ItemManager.GiveItem` _itemmanager (`self.GenerateRandomItem`)))))

(fn `UserConstructionScript`
  (`parent.UserConstructionScript`))