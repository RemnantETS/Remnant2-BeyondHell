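; Base trait tome pickup in the Boss Rush quest's item manager that awards traits to players.
; On pickup, it adds a BP_TraitTome_Base item to every other player's inventory before running the parent pickup logic.
; On award, it soft-loads trait classes from the cached spawn list, then unlocks each, grants a point and purchases it on the owner's traits component.
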(event `self.OnPickedUp`
  (params (Inventory :type "InventoryComponent Object Reference"))
  (`self.SharePickup` Inventory)
  (`parent.OnPickedUp` Inventory))

(fn `ApplyTrait`
  (params (Traits :type "TraitsComponent Object Reference") (TraitBP :type "Trait Class Reference"))
  (`TraitsComponent.K2_UnlockTraitSoft` :`self` Traits :`TraitBP` (`|ConvertAsset` TraitBP) :`StartingLevel` -1 :`bAllowAutoEquip` true)
  (`TraitsComponent.AddTraitPoints` Traits 1 false)
  (`TraitsComponent.Purchase` Traits TraitBP))

(fn `GetControllerFromInventoryComponent`
  (params (Inventory :type "InventoryComponent Object Reference"))
  (returns (Controller :type "PlayerController Object Reference"))
  (bind _asremnant_character (cast `RemnantCharacter` (`ActorComponent.GetOwner` Inventory)))
  (bind _asplayer_controller (cast `PlayerController` (`Pawn.GetController` _asremnant_character)))
  (return _asplayer_controller))

(fn `GetLabel`
  (returns (ReturnValue :type Text))
  (return (`|FormatText` "Trait Tome: {Book}" (`parent.GetLabel`))))

(fn `GetTraits`
  (returns (Traits :type "Array of Trait Class Reference"))
  (locals (AllAwardedTraits :type "Array of Trait Class Reference"))
  (bind _cachedspawnlist_spawns (break `SpawnList` (`self.CachedSpawnList`)))
  (for _array_element _cachedspawnlist_spawns
    (bind _asspawn_table_trait (cast `SpawnTableTrait` (`.Entry` (break `SpawnEntry` _array_element))))
    (bind _returnvalue (`AssetUtil.LoadSoftClassReference` (`SpawnTableTrait.TraitClass` _asspawn_table_trait)))
    (bind _astrait (castclass `Trait` _returnvalue))
    (`KismetArrayLibrary.Array_Add` (`local.AllAwardedTraits`) _astrait))
  (return (`local.AllAwardedTraits`)))

(fn `HandleAward`
  (params (Inventory :type "InventoryComponent Object Reference") (bForceNoSharing :type Boolean))
  (bind _traits (`self.GetTraits`))
  (for _array_element _traits
    (`self.ApplyTrait` (`self.GetComponentByClass` (`ActorComponent.GetOwner` Inventory) "/Script/Remnant.RemnantTraitsComponent") _array_element))
  (return))

(fn `SharePickup`
  (params (PickupInventory :type "InventoryComponent Object Reference"))
  (bind _returnvalue (`GameUtil.GetPlayerControllers`))
  (for _array_element _returnvalue
    (if (!= _array_element (`self.GetControllerFromInventoryComponent` PickupInventory))
      (bind _asremnant_player_controller (cast `RemnantPlayerController` _array_element))
      (bind _asremnant_character (cast `RemnantCharacter` (`Controller.K2_GetPawn` _asremnant_player_controller)))
      (`InventoryComponent.K2_AddItem` (`RemnantCharacter.Inventory` _asremnant_character) "BP_TraitTome_Base_C" 1 0 "PickedUp" false))))

(fn `UserConstructionScript`)