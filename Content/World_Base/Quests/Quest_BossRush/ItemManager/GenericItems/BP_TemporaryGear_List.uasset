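; Boss Rush pickup that awards one random piece of temporary gear from its RandomLoot list.
; GenerateItem rolls once and caches the result, which feeds the interact label and icon at construction and the cached spawn list, built before and after parent BeginPlay.
; HandleAward registers the item with the item manager of the inventory's owner, adds it to the inventory, sends the pickup notification, then calls the parent.
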(event `self.ReceiveBeginPlay`
  (bind _out (`self.GenerateItem`))
  (`|ExecutionSequence`
    (:`then_0`
      (bind _returnvalue (`AssetUtil.LoadSoftClassReference` _out :!label _label))
      (bind _asitem (castclass `Item` _returnvalue))
      (set `self.CachedSpawnList` (make `SpawnList` (`|MakeArray` (make `SpawnEntry` :`Type` "Item" :`ActorBP` _out :`CachedActorBP` _asitem :`Quantity` 1 :`SpawnFlags` 6)))))
    (:`then_1`
      (`parent.ReceiveBeginPlay`))
    (:`then_2`
      (goto _label))))

(fn `GenerateItem`
  (returns (Out :type "Item Soft Class Reference"))
  (if (not (`KismetSystemLibrary.IsValidSoftClassReference` (`self.GeneratedItem`)))
    (bind _output_get (set `self.GeneratedItem` (`KismetArrayLibrary.Array_Random` (`self.RandomLoot`)))))
  (return _output_get))

(fn `HandleAward`
  (params (Inventory :type "InventoryComponent Object Reference") (bForceNoSharing :type Boolean))
  (bind _generateditem (`self.GeneratedItem`))
  (bind _returnvalue (`AssetUtil.LoadSoftClassReference` _generateditem))
  (bind _asitem (castclass `Item` _returnvalue))
  (bind _itemmanager (`self.GetItemManager` (`ActorComponent.GetOwner` Inventory)))
  (`/Game/World_Base/Quests/Quest_BossRush/ItemManager/Action_Temporary_ItemManager.RegisterItem` _itemmanager _asitem)
  (`InventoryComponent.K2_AddItemSoft` :`self` Inventory :`ItemBP` _generateditem :`Quantity` 1 :`Reason` "PickedUp")
  (`InventoryComponent.RouteNotifyPickupItem` Inventory _asitem 1 0 "PickedUp")
  (`parent.HandleAward` Inventory bForceNoSharing))

(fn `UserConstructionScript`
  (`|ExecutionSequence`
    (:`then_0`
      (bind _returnvalue (`AssetUtil.LoadSoftClassReference` (`self.GenerateItem`)))
      (bind _asitem (castclass `Item` _returnvalue))
      (`|ExecutionSequence`
        (:`then_0`
          (bind (_type _category _filtertags _maxstackcount _basemaxquantity _maxquantitybonusstat _maxquantitymultiplierstat _keepininventorywithnoquantity _stats _unique _bneedsquantitytoselect _label _sublabel _description _pickupdescription _flavortext _icon) (defaults `Object` _asitem))
          (bind _output_get (set `self.Label` _label))
          (set `self.InteractLabel` _output_get))
        (:`then_1`
          (bind _output_get_2 (set `self.Icon` _icon))
          (set `self.InteractIcon` _output_get_2))))
    (:`then_1`
      (`parent.UserConstructionScript`))))