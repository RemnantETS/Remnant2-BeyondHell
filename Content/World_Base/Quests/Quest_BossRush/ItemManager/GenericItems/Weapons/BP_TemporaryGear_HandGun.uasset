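; BP_TemporaryGear_HandGun is a temporary handgun gear item in the Boss Rush quest's generic weapon items.
; GenerateItem rolls BossChance to choose between the RandomBossLoot and RandomLoot pools, then picks a random soft class from that pool.
; The pick is stored in GeneratedItem and reused on later calls while that reference stays valid.
; The event graph holds only disabled stubs, and construction just calls the parent.
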(fn `GenerateItem`
  (returns (Out :type "Item Soft Class Reference"))
  (if (not (`KismetSystemLibrary.IsValidSoftClassReference` (`self.GeneratedItem`)))
    (bind _output_get (set `self.GeneratedItem` (`KismetArrayLibrary.Array_Random` (select `bool` (`KismetMathLibrary.RandomBoolWithWeight` (`self.BossChance`)) :`false` (`self.RandomLoot`) :`true` (`self.RandomBossLoot`))))))
  (return _output_get))

(fn `UserConstructionScript`
  (`parent.UserConstructionScript`))